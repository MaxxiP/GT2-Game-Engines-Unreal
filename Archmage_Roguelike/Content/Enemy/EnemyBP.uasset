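; Enemy actor that chases the player character on sight and has its own Health value.
; PawnSensing filters seen pawns to CharacterBP and sends the enemy toward them with AIMoveTo.
; A B key press, apparently a damage test, lowers the enemy's own Health through DecreaseHealth.
; At zero or below, it shows the GameOverWidget and mouse cursor, pauses the game and destroys itself.
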(event OnSeePawn(PawnSensing)
  (params (Pawn :type Pawn%20Object%20Reference))
  (bind _ascharacter_bp (Utilities|Casting|CastToCharacterBP Pawn))
  (AI|AIMoveTo self "0, 0, 0" _ascharacter_bp 5.0 false))

(event EventBeginPlay)

(event Collision|EventActorBeginOverlap
  (params (OtherActor :type Actor%20Object%20Reference)))

(event EventTick
  (params (DeltaSeconds :type Float%20%28single-precision%29)))

(event Input|KeyboardEvents|B
  (params (Key :type Key%20Structure :default "None"))
  ;[1 1 1] Deal Damage to Character
  (:Pressed
    (Variables|Default|SetDamage 50)
    (CallFunction|DecreaseHealth)
    (if (<= (Variables|Default|GetHealth) 0)
      (bind _returnvalue (UserInterface|CreateWidget "/Game/GameOver/GameOverWidget.GameOverWidget_C"))
      (UserInterface|Viewport|AddtoViewport _returnvalue 0)
      (Variables|/Script/Engine.PlayerController|SetbShowMouseCursor (Game|GetPlayerController 0) true)
      (Game|SetGamePaused true)
      (Actor|DestroyActor))))

(fn ConstructionScript)

(fn DecreaseHealth
  (Variables|Default|SetHealth (- (Variables|Default|GetHealth) (Variables|Default|GetDamage))))